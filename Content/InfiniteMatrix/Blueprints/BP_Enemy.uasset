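; BP_Enemy is an enemy actor that bobs vertically, damages the player on contact and can be shot for score.
; Each Tick moves the Enemy component by a Z delta that ramps between -15 and 15, reversing at the limits, independent of delta time.
; On hit, it destroys itself and either reduces BP_Player health, showing restart at zero, or shortens the BP_Projectile lifespan and increments the player's score.
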(event OnComponentHit(Enemy)
  (params (HitComponent :type Primitive%20Component%20Object%20Reference) (OtherActor :type Actor%20Object%20Reference) (OtherComp :type Primitive%20Component%20Object%20Reference) (NormalImpulse :type Vector :default "0, 0, 0") (Hit :type Hit%20Result%20Structure%20%28by%20ref%29))
  (bind _asbp_player (Utilities|Casting|CastToBP_Player OtherActor)
    (:then
      (Utilities|FlowControl|Sequence
        (:then_0
          (Actor|DestroyActor))
        (:then_1
          (bind _output_get (Variables|/Game/InfiniteMatrix/Blueprints/BP_Player.BP_Player_C|SetHealth _asbp_player (Math|Float|Clamp(Float) (- (Variables|/Game/InfiniteMatrix/Blueprints/BP_Player.BP_Player_C|GetHealth _asbp_player) 2e+01) 0.0 1e+02)))
          (if (== _output_get 0.0)
            (Variables|/Game/InfiniteMatrix/Blueprints/BP_Player.BP_Player_C|SetisDead _asbp_player true)
            (Default|DisplayRestart _asbp_player)))))
    (:CastFailed
      (bind _asbp_projectile (Utilities|Casting|CastToBP_Projectile OtherActor))
      (Actor|DestroyActor)
      (Actor|SetLifeSpan _asbp_projectile 0.2)
      (bind _returnvalue (Actor|GetActorOfClass "/Game/InfiniteMatrix/Blueprints/BP_Player.BP_Player_C"))
      (Variables|/Game/InfiniteMatrix/Blueprints/BP_Player.BP_Player_C|Setscore _returnvalue (+ (Variables|/Game/InfiniteMatrix/Blueprints/BP_Player.BP_Player_C|Getscore _returnvalue) 1)))))

(event EventTick
  (params (DeltaSeconds :type Float%20%28single-precision%29))
  (Utilities|FlowControl|Sequence
    (:then_0
      (bind _output_get (Variables|Default|SetzTransform (+ (Variables|Default|GetzTransform) (Variables|Default|Getdirection))))
      (Class|SceneComponent|AddLocalTransform (Variables|Default|GetEnemy) (Math|Transform|MakeTransform (Math|Vector|MakeVector 0.0 0.0 _output_get) "0, 0, 0" "1.000000,1.000000,1.000000") false false))
    (:then_1
      (if (>= (Variables|Default|GetzTransform) 15.0)
        (Variables|Default|Setdirection -1.0)
        (elif (<= (Variables|Default|GetzTransform) -15.0)
          (Variables|Default|Setdirection 1.0))))))

(fn ConstructionScript)