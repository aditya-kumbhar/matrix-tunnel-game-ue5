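; BP_EnemySpawner is an actor that manages BP_Enemy instances along the X axis relative to BP_Player.
; SpawnRandomEnemy first destroys every enemy with a lower X than the player, then has a one-in-five chance to spawn a scaled-down enemy at a random distance ahead, with random Y and Z within fixed bands.
; Its own event graph is empty, so the function runs only when called externally.
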(event EventBeginPlay)

(event Collision|EventActorBeginOverlap
  (params (OtherActor :type Actor%20Object%20Reference)))

(event EventTick
  (params (DeltaSeconds :type Float%20%28single-precision%29)))

(fn ConstructionScript)

(fn SpawnRandomEnemy
  (Utilities|FlowControl|Sequence
    (:then_0
      (bind _returnvalue (Actor|GetActorOfClass "/Game/InfiniteMatrix/Blueprints/BP_Player.BP_Player_C"))
      (bind _outactors (Actor|GetAllActorsOfClass "/Game/InfiniteMatrix/Blueprints/BP_Enemy.BP_Enemy_C"))
      (for _array_element _outactors
        (if (< (.x (Transformation|GetActorLocation _array_element)) (.x (Transformation|GetActorLocation _returnvalue)))
          (Actor|DestroyActor _array_element))))
    (:then_1
      (if (== (Math|Random|RandomInteger 5) 0)
        (bind _returnvalue_2 (Actor|GetActorOfClass "/Game/InfiniteMatrix/Blueprints/BP_Player.BP_Player_C"))
        (Game|SpawnActorfromClass "/Game/InfiniteMatrix/Blueprints/BP_Enemy.BP_Enemy_C" (Math|Transform|MakeTransform (Math|Vector|MakeVector (+ (.x (Transformation|GetActorLocation _returnvalue_2)) (Math|Random|RandomFloatinRange 3.2e+03 4.5e+03)) (Math|Random|RandomFloatinRange -2.5e+02 2.5e+02) (Math|Random|RandomFloatinRange -1e+02 1e+02)) "0, 0, 0" "0.600000,0.600000,0.600000") "Undefined" 0 0)))))