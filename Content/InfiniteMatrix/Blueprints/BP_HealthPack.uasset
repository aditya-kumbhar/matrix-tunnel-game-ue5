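; BP_HealthPack is a spinning pickup that restores 20 health to the player.
; It rotates its HealthPack component by a fixed step each tick, independent of delta time.
; When that component is hit by a BP_Player, it destroys itself and adds the health, clamped between 0 and 100.
; It then finds HealthWidget instances through GetAllWidgetsOfClass and animates their health bar to the new value.
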(event OnComponentHit(HealthPack)
  (params (HitComponent :type Primitive%20Component%20Object%20Reference) (OtherActor :type Actor%20Object%20Reference) (OtherComp :type Primitive%20Component%20Object%20Reference) (NormalImpulse :type Vector :default "0, 0, 0") (Hit :type Hit%20Result%20Structure%20%28by%20ref%29))
  (bind _asbp_player (Utilities|Casting|CastToBP_Player OtherActor))
  (Utilities|FlowControl|Sequence
    (:then_0
      (Actor|DestroyActor))
    (:then_1
      (bind _output_get (Variables|/Game/InfiniteMatrix/Blueprints/BP_Player.BP_Player_C|SetHealth _asbp_player (Math|Float|Clamp(Float) (+ (Variables|/Game/InfiniteMatrix/Blueprints/BP_Player.BP_Player_C|GetHealth _asbp_player) 2e+01) 0.0 1e+02)))
      (bind _foundwidgets (Widget|GetAllWidgetsOfClass "/Game/InfiniteMatrix/UI/HealthWidget.HealthWidget_C" true))
      (Default|AnimateHealthbar _foundwidgets _output_get))))

(event EventBeginPlay)

(event Collision|EventActorBeginOverlap
  (params (OtherActor :type Actor%20Object%20Reference)))

(event EventTick
  (params (DeltaSeconds :type Float%20%28single-precision%29))
  (Transformation|AddLocalRotation (Variables|Default|GetHealthPack) "0.000000,5.000000,0.000000" false false))

(fn ConstructionScript)