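; BP_HealthPackSpawner spawns health pickups ahead of the player along the X axis.
; RandomSpawnHealthPack first destroys every BP_HealthPack behind the player, then has a one-in-four chance to call SpawnHealthPack at a random point ahead, offset in Y and Z.
; SpawnHealthPack creates the pack at half scale.
; BeginPlay is empty, so the spawn routine relies on an outside caller.
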(event EventBeginPlay)

(fn ConstructionScript)

(fn SpawnHealthPack
  (params (SpawnLocation :type Vector))
  (Game|SpawnActorfromClass "/Game/InfiniteMatrix/Blueprints/BP_HealthPack.BP_HealthPack_C" (Math|Transform|MakeTransform SpawnLocation "0, 0, 0" "0.500000,0.500000,0.500000") "Undefined" 0 0))

(fn RandomSpawnHealthPack
  (Utilities|FlowControl|Sequence
    (:then_0
      (bind _returnvalue (Actor|GetActorOfClass "/Game/InfiniteMatrix/Blueprints/BP_Player.BP_Player_C"))
      (bind _outactors (Actor|GetAllActorsOfClass "/Game/InfiniteMatrix/Blueprints/BP_HealthPack.BP_HealthPack_C"))
      (for _array_element _outactors
        (if (< (.x (Transformation|GetActorLocation _array_element)) (.x (Transformation|GetActorLocation _returnvalue)))
          (Actor|DestroyActor _array_element))))
    (:then_1
      (if (== (Math|Random|RandomInteger 4) 0)
        (bind _returnvalue_2 (Actor|GetActorOfClass "/Game/InfiniteMatrix/Blueprints/BP_Player.BP_Player_C"))
        (CallFunction|SpawnHealthPack (Math|Vector|MakeVector (+ (.x (Transformation|GetActorLocation _returnvalue_2)) (Math|Random|RandomFloatinRange 3e+03 4.7e+03)) (Math|Random|RandomFloatinRange -2.5e+02 2.5e+02) (Math|Random|RandomFloatinRange -2e+02 -7e+02)))))))