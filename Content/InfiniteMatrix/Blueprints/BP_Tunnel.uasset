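; BP_Tunnel is an endless-runner tunnel segment with a rotating holed wall, whose mesh and roll RandomizeWall randomizes.
; When the player overlaps TriggerZone, it requests a new tunnel, destroys itself, adds score with periodic speed boosts, and triggers health pack and enemy spawners.
; Hitting the wall damages the player, either showing restart on death or replacing the segment and animating the health bar; projectiles are destroyed on impact.
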(event OnComponentHit(WallMesh)
  (params (HitComponent :type Primitive%20Component%20Object%20Reference) (OtherActor :type Actor%20Object%20Reference) (OtherComp :type Primitive%20Component%20Object%20Reference) (NormalImpulse :type Vector :default "0, 0, 0") (Hit :type Hit%20Result%20Structure%20%28by%20ref%29))
  (bind _asbp_player (Utilities|Casting|CastToBP_Player OtherActor)
    (:then
      (bind _output_get (Variables|/Game/InfiniteMatrix/Blueprints/BP_Player.BP_Player_C|SetHealth _asbp_player (Math|Float|Clamp(Float) (- (Variables|/Game/InfiniteMatrix/Blueprints/BP_Player.BP_Player_C|GetHealth _asbp_player) 2e+01) 0.0 (Variables|/Game/InfiniteMatrix/Blueprints/BP_Player.BP_Player_C|GetMaxHealth _asbp_player))))
      (if (== _output_get 0.0)
        (Variables|/Game/InfiniteMatrix/Blueprints/BP_Player.BP_Player_C|SetisDead _asbp_player true)
        (Default|DisplayRestart _asbp_player)
        (else
          (Utilities|FlowControl|Sequence
            (:then_0
              (Default|SpawnTunnelatSpawnPoint (Variables|Default|GetTunnelSpawner))
              (Actor|DestroyActor))
            (:then_1
              (bind _foundwidgets (Widget|GetAllWidgetsOfClass "/Game/InfiniteMatrix/UI/HealthWidget.HealthWidget_C" true))
              (Default|AnimateHealthbar _foundwidgets _output_get))))))
    (:CastFailed
      (bind _asbp_projectile (Utilities|Casting|CastToBP_Projectile OtherActor))
      (Actor|DestroyActor _asbp_projectile))))

(event OnComponentBeginOverlap(TriggerZone)
  (params (OverlappedComponent :type Primitive%20Component%20Object%20Reference) (OtherActor :type Actor%20Object%20Reference) (OtherComp :type Primitive%20Component%20Object%20Reference) (OtherBodyIndex :type Integer) (bFromSweep :type Boolean) (SweepResult :type Hit%20Result%20Structure%20%28by%20ref%29))
  (bind _asbp_player (Utilities|Casting|CastToBP_Player OtherActor))
  (Utilities|FlowControl|Sequence
    (:then_0
      (Default|SpawnTunnelatSpawnPoint (Variables|Default|GetTunnelSpawner))
      (Actor|DestroyActor))
    (:then_1
      (bind _output_get (Variables|/Game/InfiniteMatrix/Blueprints/BP_Player.BP_Player_C|Setscore _asbp_player (+ (Variables|/Game/InfiniteMatrix/Blueprints/BP_Player.BP_Player_C|Getscore _asbp_player) 1)))
      (if (== (Math|Integer|%(Integer) (Math|Conversions|ToInteger(Byte) _output_get) 5) 0)
        (Variables|/Game/InfiniteMatrix/Blueprints/BP_Player.BP_Player_C|SetForwardSpeed _asbp_player (Math|Float|Clamp(Float) (+ (Variables|/Game/InfiniteMatrix/Blueprints/BP_Player.BP_Player_C|GetForwardSpeed _asbp_player) 2e+02) 0.0 3.5e+03))))
    (:then_2
      (bind _returnvalue (Actor|GetActorOfClass "/Game/InfiniteMatrix/Blueprints/BP_HealthPackSpawner.BP_HealthPackSpawner_C"))
      (Default|RandomSpawnHealthPack _returnvalue))
    (:then_3
      (bind _returnvalue_2 (Actor|GetActorOfClass "/Game/InfiniteMatrix/Blueprints/BP_EnemySpawner.BP_EnemySpawner_C"))
      (for _index (range 0 (Math|Random|RandomIntegerinRange 1 6))
        (Default|SpawnRandomEnemy _returnvalue_2)))))

(event EventBeginPlay)

(event EventTick
  (params (DeltaSeconds :type Float%20%28single-precision%29))
  (Transformation|AddLocalRotation (Variables|Default|GetWallMesh) (Math|Rotator|MakeRotator (* DeltaSeconds (Variables|Default|GetRotateSpeed)) 0.0 0.0) false false))

(fn ConstructionScript)

(fn RandomizeWall
  (Components|StaticMesh|SetStaticMesh (Variables|Default|GetWallMesh) (Utilities|Select :Index (Math|Random|RandomIntegerinRange 0 3) :Option%200 "/Game/InfiniteMatrix/Meshes/SM_Hole_01.SM_Hole_01" :Option%201 "/Game/InfiniteMatrix/Meshes/SM_Hole_02.SM_Hole_02" :Option%202 "/Game/InfiniteMatrix/Meshes/SM_Hole_03.SM_Hole_03" :Option%203 "/Game/InfiniteMatrix/Meshes/SM_Hole_04.SM_Hole_04"))
  (Transformation|AddLocalRotation (Variables|Default|GetWallMesh) (Math|Rotator|MakeRotator (Math|Random|RandomFloatinRange 0.0 3.6e+02) 0.0 0.0) false false))

(fn RandomizeHealthPack
  (if (== (Math|Random|RandomInteger 2) 1)
    _))